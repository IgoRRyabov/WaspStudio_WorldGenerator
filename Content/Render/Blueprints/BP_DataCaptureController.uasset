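; Data capture controller that renders a level sequence through Movie Render Queue at runtime with a requested resolution and file name.
; StartRenderImage allocates a queue job from a preset configuration and overrides its output setting.
; It then renders the queue with an in-process executor using the current level.
; RenderEnd prints the result and calls NotifyRenderFinished only on success.
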(event `self.StartRenderImage`
  (params (PC :type "MyPC Object Reference") (InRenderW :type Integer) (InRenderH :type Integer) (FrameBaseName :type String))
  (bind _returnvalue (subsystem `MoviePipelineQueueEngineSubsystem`))
  (set `self.In Render W` InRenderW)
  (set `self.In Render H` InRenderH)
  (set `self.Frame Base Name` FrameBaseName)
  (`|ExecutionSequence`
    (:`then_0`
      (bind _returnvalue_2 (`MoviePipelineQueueEngineSubsystem.AllocateJob` (subsystem `MoviePipelineQueueEngineSubsystem`) "/Game/Render/LSequance.LSequance"))
      (`MoviePipelineExecutorJob.SetConfiguration` _returnvalue_2 "/Game/Render/MySettingRender.MySettingRender")
      (bind _returnvalue_3 (`MoviePipelineConfigBase.FindOrAddSettingByClass` (`MoviePipelineExecutorJob.GetConfiguration` _returnvalue_2) "/Script/MovieRenderPipelineCore.MoviePipelineOutputSetting" false false))
      (set `MoviePipelineOutputSetting.OutputResolution` (make `IntPoint` (`self.In Render W`) (`self.In Render H`)) _returnvalue_3)
      (set `MoviePipelineOutputSetting.FileNameFormat` (`self.Frame Base Name`) _returnvalue_3))
    (:`then_1`
      (bind _returnvalue_4 (`|GenericCreateObject` _returnvalue "/Script/MovieRenderPipelineCore.MoviePipelineInProcessExecutor"))
      (set `MoviePipelineInProcessExecutor.bUseCurrentLevel` true _returnvalue_4)
      (add `MoviePipelineExecutorBase.OnExecutorFinishedDelegate` _returnvalue_4 (delegate `RenderEnd`))
      (`MoviePipelineQueueEngineSubsystem.RenderQueueWithExecutorInstance` _returnvalue _returnvalue_4))))

(event `RenderEnd`
  (params (PipelineExecutor :type "MoviePipelineExecutorBase Object Reference") (bSuccess :type Boolean))
  (if bSuccess
    (`KismetSystemLibrary.PrintString` "RenderSuccess")
    (`self.NotifyRenderFinished`)
    (else
      (`KismetSystemLibrary.PrintString` "RenderError"))))

(fn `UserConstructionScript`)