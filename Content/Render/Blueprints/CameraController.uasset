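; Camera controller that orbits a camera around a tank target for ten timed shots and records its screen-space bounding box, then quits.
; BeginPlay caches camera, target and player controller; TakeShot, not triggered here, re-calls itself after each delay.
; Each shot steps evenly around an elevated circle, adding random position and aim noise.
; Eight bounds corners, passed through the target's transform, are projected to screen, and their min/max written to BP_PlayerController.
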(event `self.ReceiveBeginPlay`
  (bind _returnvalue (`GameplayStatics.GetActorOfClass` "/Script/Engine.CameraActor"))
  (set `self.CameraActor` _returnvalue)
  (bind _returnvalue_2 (`GameplayStatics.GetActorOfClass` "/Game/Render/Blueprints/TargetActor.TargetActor_C"))
  (set `self.Tank` _returnvalue_2)
  (bind _output_get (set `self.ControllreRef` (`GameplayStatics.GetPlayerController` 0))))

(event `TakeShot`
  (set `self.Angle` (/ (* (`self.ShotIndex`) 360) 10))
  (`self.PlaceCameraOnCircleWithNoise` (`self.CameraActor`) (`self.Tank`) (`self.Radius`) 5000.0 (`self.Angle`) 100.0 8.0)
  (set `self.ShotIndex` (+ (`self.ShotIndex`) 1))
  (bind (_minxout _minyout _maxxout _maxyout) (`self.GetObjectScreenBoundingBox` (`self.Tank`) (`self.ControllreRef`)))
  (bind _asbp_player_controller (cast `/Game/Render/Blueprints/BP_PlayerController` (`self.ControllreRef`)))
  (set `/Game/Render/Blueprints/BP_PlayerController.MinX` _minxout _asbp_player_controller)
  (set `/Game/Render/Blueprints/BP_PlayerController.MinY` _minyout _asbp_player_controller)
  (set `/Game/Render/Blueprints/BP_PlayerController.MaxX` _maxxout _asbp_player_controller)
  (set `/Game/Render/Blueprints/BP_PlayerController.MaxY` _maxyout _asbp_player_controller)
  (if (< (`self.ShotIndex`) 10)
    (`KismetSystemLibrary.Delay` 4.0)
    (`self.TakeShot`)
    (else
      (`KismetSystemLibrary.Delay` 4.0)
      (`KismetSystemLibrary.QuitGame` null "Quit"))))

(fn `GetObjectScreenBoundingBox`
  (params (TargetActor :type "Actor Object Reference") (Controller :type "PlayerController Object Reference"))
  (returns (MinXOut :type "Float (double-precision)") (MinYOut :type "Float (double-precision)") (MaxXOut :type "Float (double-precision)") (MaxYOut :type "Float (double-precision)"))
  (locals (Origin :type "Vector Structure") (BoxExtent :type "Vector Structure") (Corners :type "Array of Vector Structure") (MinX :type "Float (double-precision)") (MinY :type "Float (double-precision)") (MaxX :type "Float (double-precision)") (MaxY :type "Float (double-precision)") (ControllerTemp :type "PlayerController Object Reference") (ScreenPosition :type "Vector2D Structure") (SX :type "Float (double-precision)") (SY :type "Float (double-precision)") (TargetActorRef :type "Actor Object Reference") (WorldCorners :type "Array of Vector Structure"))
  (bind (_origin _boxextent) (`self.GetActorBounds` TargetActor false false))
  (bind (_boxextent_x _boxextent_y _boxextent_z) (`KismetMathLibrary.BreakVector` (`local.BoxExtent`)))
  (bind (_boxextent_x_2 _boxextent_y_2 _boxextent_z_2) (`KismetMathLibrary.BreakVector` (`local.BoxExtent`)))
  (bind (_boxextent_x_3 _boxextent_y_3 _boxextent_z_3) (`KismetMathLibrary.BreakVector` (`local.BoxExtent`)))
  (bind (_boxextent_x_4 _boxextent_y_4 _boxextent_z_4) (`KismetMathLibrary.BreakVector` (`local.BoxExtent`)))
  (bind (_boxextent_x_5 _boxextent_y_5 _boxextent_z_5) (`KismetMathLibrary.BreakVector` (`local.BoxExtent`)))
  (bind (_boxextent_x_6 _boxextent_y_6 _boxextent_z_6) (`KismetMathLibrary.BreakVector` (`local.BoxExtent`)))
  (bind (_boxextent_x_7 _boxextent_y_7 _boxextent_z_7) (`KismetMathLibrary.BreakVector` (`local.BoxExtent`)))
  (bind (_boxextent_x_8 _boxextent_y_8 _boxextent_z_8) (`KismetMathLibrary.BreakVector` (`local.BoxExtent`)))
  (set `local.TargetActorRef` TargetActor)
  (set `self.ControllreRef` Controller)
  (set `local.Origin` _origin)
  (set `local.BoxExtent` _boxextent)
  (bind _output_get (set `local.Corners` (`|MakeArray` (`KismetMathLibrary.MakeVector` _boxextent_x_2 _boxextent_y_2 _boxextent_z_2) (`KismetMathLibrary.MakeVector` _boxextent_x_3 _boxextent_y_3 (* _boxextent_z_3 -1.0)) (`KismetMathLibrary.MakeVector` _boxextent_x_4 (* _boxextent_y_4 -1.0) _boxextent_z_4) (`KismetMathLibrary.MakeVector` _boxextent_x_5 (* _boxextent_y_5 -1.0) (* _boxextent_z_5 -1.0)) (`KismetMathLibrary.MakeVector` (* _boxextent_x_6 -1.0) _boxextent_y_6 _boxextent_z_6) (`KismetMathLibrary.MakeVector` (* _boxextent_x_7 -1.0) _boxextent_y_7 (* _boxextent_z_7 -1.0)) (`KismetMathLibrary.MakeVector` (* _boxextent_x_8 -1.0) (* _boxextent_y_8 -1.0) _boxextent_z_8) (`KismetMathLibrary.MakeVector` (* _boxextent_x -1.0) (* _boxextent_y -1.0) (* _boxextent_z -1.0)))))
  (for (_array_element _array_index) _output_get
    (`KismetArrayLibrary.Array_Set` (`local.WorldCorners`) _array_index (`KismetMathLibrary.TransformLocation` (`self.GetTransform` (`local.TargetActorRef`)) _array_element)))
  (set `local.MinX` 999999.0)
  (set `local.MinY` 999999.0)
  (set `local.MaxX` -999999.0)
  (set `local.MaxY` -999999.0)
  (for _array_element_2 (`local.WorldCorners`)
    (bind _output_get_2 (set `local.ScreenPosition` (`GameplayStatics.ProjectWorldToScreen` (`self.ControllreRef`) _array_element_2)))
    (set `local.SX` (`KismetMathLibrary.BreakVector2D` _output_get_2))
    (set `local.SY` (`.Y` (`KismetMathLibrary.BreakVector2D` _output_get_2)))
    (set `local.MinX` (`KismetMathLibrary.SelectFloat` (`local.SX`) (`local.MinX`) (< (`local.SX`) (`local.MinX`))))
    (set `local.MaxX` (`KismetMathLibrary.SelectFloat` (`local.SX`) (`local.MaxX`) (> (`local.SX`) (`local.MaxX`))))
    (set `local.MinY` (`KismetMathLibrary.SelectFloat` (`local.SY`) (`local.MinY`) (< (`local.SY`) (`local.MinY`))))
    (set `local.MaxY` (`KismetMathLibrary.SelectFloat` (`local.SY`) (`local.MaxY`) (> (`local.SY`) (`local.MaxY`)))))
  (return (`local.MinX`) (`local.MinY`) (`local.MaxX`) (`local.MaxY`)))

(fn `PlaceCameraOnCircleWithNoise`
  (params (`Camera Ref` :type "CameraActor Object Reference") (TargetActor :type "Actor Object Reference") (Radius :type "Float (double-precision)") (HeightOffset :type "Float (double-precision)") (AngleDeg :type "Float (double-precision)") (PositionNoise :type "Float (double-precision)") (AimNoiseDeg :type "Float (double-precision)"))
  (locals (Center :type "Vector Structure" :default (0.0 0.0 0.0)) (RadiusTemp :type "Float (double-precision)") (AngleRad :type "Float (double-precision)" :default 0.0) (X :type "Float (double-precision)") (Y :type "Float (double-precision)") (Z :type "Float (double-precision)") (BaseCameraLocation :type "Vector Structure") (PositionNoiseTemp :type "Float (double-precision)") (NoiseX :type "Float (double-precision)") (NoiseY :type "Float (double-precision)") (NoiseZ :type "Float (double-precision)") (NoiseLocation :type "Vector Structure") (LookRot :type "Rotator Structure") (AimPitchNoise :type "Float (double-precision)") (AimYawNoise :type "Float (double-precision)") (AimNoiseDegTemp :type "Float (double-precision)") (CameraRefTemp :type "CameraActor Object Reference"))
  (bind (_center_x _center_y _center_z) (`KismetMathLibrary.BreakVector` (`local.Center`)))
  (bind _center_x_2 (`KismetMathLibrary.BreakVector` (`local.Center`)))
  (bind (_center_x_3 _center_y_2) (`KismetMathLibrary.BreakVector` (`local.Center`)))
  (set `local.CameraRefTemp` `Camera Ref`)
  (set `local.AimNoiseDegTemp` AimNoiseDeg)
  (set `local.PositionNoiseTemp` PositionNoise)
  (set `local.RadiusTemp` Radius)
  (set `local.Center` (`self.K2_GetActorLocation` TargetActor))
  (set `local.AngleRad` (`KismetMathLibrary.DegreesToRadians` AngleDeg))
  (set `local.X` (+ (* (`local.RadiusTemp`) (`KismetMathLibrary.Cos` (`local.AngleRad`))) _center_x_2))
  (set `local.Y` (+ (* (`local.RadiusTemp`) (`KismetMathLibrary.Sin` (`local.AngleRad`))) _center_y_2))
  (set `local.Z` (+ HeightOffset _center_z))
  (set `local.BaseCameraLocation` (`KismetMathLibrary.MakeVector` (`local.X`) (`local.Y`) (`local.Z`)))
  (set `local.NoiseX` (`KismetMathLibrary.RandomFloatInRange` (* (`local.PositionNoiseTemp`) -1.0) (`local.PositionNoiseTemp`)))
  (set `local.NoiseY` (`KismetMathLibrary.RandomFloatInRange` (* (`local.PositionNoiseTemp`) -1.0) (`local.PositionNoiseTemp`)))
  (set `local.NoiseZ` (`KismetMathLibrary.RandomFloatInRange` (* (`local.PositionNoiseTemp`) -1.0) (`local.PositionNoiseTemp`)))
  (set `local.NoiseLocation` (+ (`local.BaseCameraLocation`) (`KismetMathLibrary.MakeVector` (`local.NoiseX`) (`local.NoiseY`) (`local.NoiseZ`))))
  (set `local.LookRot` (`KismetMathLibrary.FindLookAtRotation` (`local.NoiseLocation`) (`local.Center`)))
  (set `local.AimPitchNoise` (`KismetMathLibrary.RandomFloatInRange` (* (`local.AimNoiseDegTemp`) -1.0) (`local.AimNoiseDegTemp`)))
  (set `local.AimYawNoise` (`KismetMathLibrary.RandomFloatInRange` (* (`local.AimNoiseDegTemp`) -1.0) (`local.AimNoiseDegTemp`)))
  (set `local.LookRot` (`KismetMathLibrary.MakeRotator` 0.0 (+ (.pitch (`local.LookRot`)) (`local.AimPitchNoise`)) (+ (.yaw (`local.LookRot`)) (`local.AimYawNoise`))))
  (`self.K2_SetActorLocation` (`local.CameraRefTemp`) (`local.NoiseLocation`) false false)
  (`self.K2_SetActorRotation` (`local.CameraRefTemp`) (`local.LookRot`) false))

(fn `UserConstructionScript`)