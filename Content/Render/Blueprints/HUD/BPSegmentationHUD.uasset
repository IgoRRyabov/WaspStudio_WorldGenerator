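; BPSegmentationHUD is a HUD Blueprint that draws a filled screen-space rectangle from bounds held by BP_PlayerController.
; Each DrawHUD call casts the first player controller, reads its min and max X/Y, and converts them to origin, width and height for DrawRect in the HUD's Color.
; It also prints the four bound values to screen every frame without logging them.
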(event `self.ReceiveDrawHUD`
  (params (SizeX :type Integer) (SizeY :type Integer))
  (bind _asbp_player_controller (cast `/Game/Render/Blueprints/BP_PlayerController` (`GameplayStatics.GetPlayerController` 0)))
  (bind _minx (`/Game/Render/Blueprints/BP_PlayerController.MinX` _asbp_player_controller))
  (`KismetSystemLibrary.PrintString` (`KismetStringLibrary.Conv_DoubleToString` _minx) true false)
  (bind _miny (`/Game/Render/Blueprints/BP_PlayerController.MinY` _asbp_player_controller))
  (`KismetSystemLibrary.PrintString` (`KismetStringLibrary.Conv_DoubleToString` _miny) true false)
  (bind _maxx (`/Game/Render/Blueprints/BP_PlayerController.MaxX` _asbp_player_controller))
  (`KismetSystemLibrary.PrintString` (`KismetStringLibrary.Conv_DoubleToString` _maxx) true false)
  (bind _maxy (`/Game/Render/Blueprints/BP_PlayerController.MaxY` _asbp_player_controller))
  (`KismetSystemLibrary.PrintString` (`KismetStringLibrary.Conv_DoubleToString` _maxy) true false)
  (`self.DrawRect` (`self.Color`) _minx _miny (- _maxx _minx) (- _maxy _miny)))

(fn `UserConstructionScript`)