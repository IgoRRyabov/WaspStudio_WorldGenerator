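; BP_MyPC is an input Blueprint that drives a data capture session through the level's BP_DataCaptureController, which it finds and caches on BeginPlay.
; Releasing F sets CanRender and starts the capture controller, while Space tells it to update its camera transform.
; Escape clears CanRender and opens MainMenuLevel, and a second Space release handler is wired into that same exit path.
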(event `self.ReceiveBeginPlay`
  (bind _returnvalue (`GameplayStatics.GetActorOfClass` "/Game/Render/Blueprints/BP_DataCaptureController.BP_DataCaptureController_C"))
  (set `self.NewVar` _returnvalue))

(event `Key|F`
  (params (Key :type "Key Structure"))
  (:`Released`
    (set `self.bCanRender` true)
    (`KismetSystemLibrary.PrintString` "Start")
    (`DataCaptureController.Start` (`self.NewVar`))))

(event `Key|SpaceBar`
  (params (Key :type "Key Structure"))
  (:`Released`
    (`DataCaptureController.UpdateCameraTransform` (`self.NewVar`))))

(event `Key|Escape`
  (params (Key :type "Key Structure"))
  (:`Released`
    (set `self.bCanRender` false :!label _label)
    (`GameplayStatics.OpenLevelBySoftObjectPtr` "/Game/Maps/MainMenu/MainMenuLevel.MainMenuLevel")))

(event `Key|SpaceBar`
  (params (Key :type "Key Structure"))
  (:`Released`
    (goto _label)))

(fn `UserConstructionScript`)